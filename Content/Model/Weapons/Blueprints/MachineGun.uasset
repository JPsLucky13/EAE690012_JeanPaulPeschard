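; Machine gun weapon Blueprint that fires one bullet projectile per Attack while ammo remains.
; Attack decrements ammo, spawns a Bullet_Blueprint at the BulletSpawnLocation component and passes it the calculated damage, possessor and a direction from the model's negated right vector.
; It binds to the bullet's attack summary, which it forwards to CallDisplayDamage for damage display.
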(event Custom|AttackSummary
  (params (AttackSummary :type String))
  ;[1 1 1] Fire the machine gun
  (Default|CallDisplayDamage AttackSummary))

(event EventBeginPlay)

(event Collision|EventActorBeginOverlap
  (params (OtherActor :type Actor%20Object%20Reference)))

(event EventTick
  (params (DeltaSeconds :type Float%20%28single-precision%29)))

(event EventAttack
  ;[1 1 1] Fire the machine gun
  (if (> (Variables|Default|GetAmmoAmount) 0)
    (Variables|Default|SetAmmoAmount (- (Variables|Default|GetAmmoAmount) 1))
    (bind _returnvalue (Game|SpawnActorfromClass "/Game/Model/Weapons/MachineGun/Bullets/Bullet_Blueprint.Bullet_Blueprint_C" (Math|Transform|MakeTransform (Transformation|GetWorldLocation (Variables|Default|GetBulletSpawnLocation)) (Transformation|GetWorldRotation (Variables|Default|GetBulletSpawnLocation)) (Variables|Default|GetBulletScale)) "AlwaysSpawn" 0 "NewEnumerator0" 0))
    (CallFunction|CalculateDamage)
    (CallFunction|GetPossessor)
    (Variables|/Game/Model/Weapons/MachineGun/Bullets/Bullet_Blueprint.Bullet_Blueprint_C|SetForwardVector _returnvalue (* (Math|Vector|GetRightVector (Variables|Default|GetMachineGunModel)) -1.0))
    (Variables|/Game/Model/Weapons/MachineGun/Bullets/Bullet_Blueprint.Bullet_Blueprint_C|SetfinalDamage _returnvalue (Variables|Default|GetfinalDamageValue))
    (Variables|/Game/Model/Weapons/MachineGun/Bullets/Bullet_Blueprint.Bullet_Blueprint_C|SetPossessor _returnvalue (Variables|Default|GetPossessor))
    (EventDispatchers|BindEventtoAttackSummary _returnvalue (delegate Custom|AttackSummary))))

(fn ConstructionScript)