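; Base weapon actor that provides the shared input, damage roll and owner lookup, with Attack and Initialize left as empty stubs.
; BeginPlay enables input and calls Initialize; left click calls Attack and fires the Attacked dispatcher only when Possessor equals "Player".
; GetPossessor sets Possessor from the attach parent's display name, and CalculateDamage stores a rounded-up random value between MinDamage and MaxDamage.
; Neither helper is called within this Blueprint.
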(event Collision|EventActorBeginOverlap
  (params (OtherActor :type Actor%20Object%20Reference)))

(event EventTick
  (params (DeltaSeconds :type Float%20%28single-precision%29)))

(event EventBeginPlay
  ;[1 1 1] Enable the input
  (Input|EnableInput (Game|GetPlayerController 0))
  (CallFunction|Initialize))

(event Input|MouseEvents|LeftMouseButton
  (params (Key :type Key%20Structure :default "AnyKey"))
  ;[1 1 1] Player Input
  (:Pressed
    (if (Utilities|Enum|Equal(Enum) (Variables|Default|GetPossessor) "Player")
      (CallFunction|Attack)
      (Default|CallAttacked))))

(fn ConstructionScript)

(fn Attack)

(fn CalculateDamage
  ;[1 1 1] Calculate the damage
  (Variables|Default|SetfinalDamageValue (Math|Conversions|ToFloat(Integer) (Math|Float|Ceil (Math|Random|RandomFloatinRange (Variables|Default|GetminDamage) (Variables|Default|GetmaxDamage))))))

(fn GetPossessor
  ;[1 1 1] Gets the possessor of the weapon
  (Variables|Default|SetPossessor (Utilities|GetDisplayName (Actor|GetAttachParentActor))))

(fn Initialize)