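; Chainsaw weapon actor that damages the player on contact through its attack trigger.
; Two events switch the trigger's collision between query-only and off, so hits register only while it is enabled.
; When an overlapping actor tagged Player casts to ThirdPersonCharacter, the chainsaw applies its max damage and calls that character's death check.
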(event OnComponentBeginOverlap(AttackTrigger)
  (params (OverlappedComponent :type Primitive%20Component%20Object%20Reference) (OtherActor :type Actor%20Object%20Reference) (OtherComp :type Primitive%20Component%20Object%20Reference) (OtherBodyIndex :type Integer) (bFromSweep :type Boolean) (SweepResult :type Hit%20Result%20Structure%20%28by%20ref%29))
  ;[1 1 1] Check if the weapon hit the player
  (if (Actor|ActorHasTag OtherActor "Player")
    (bind _asthird_person_character (Utilities|Casting|CastToThirdPersonCharacter OtherActor))
    (Default|ApplyDamage _asthird_person_character (Variables|Default|GetmaxDamage))
    (Default|CheckDeath _asthird_person_character)))

(event Custom|EnableWeaponTrigger
  ;[1 1 1] Enable weapon trigger
  (Collision|SetCollisionEnabled (Variables|Default|GetAttackTrigger) "QueryOnly"))

(event Custom|DisableWeaponTrigger
  ;[1 1 1] Disable weapon trigger
  (Collision|SetCollisionEnabled (Variables|Default|GetAttackTrigger) "NoCollision"))

(event EventBeginPlay)

(event Collision|EventActorBeginOverlap
  (params (OtherActor :type Actor%20Object%20Reference)))

(event EventTick
  (params (DeltaSeconds :type Float%20%28single-precision%29)))

(fn ConstructionScript)