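; Dragon sword weapon Blueprint that swings its blade on Attack and damages enemies it overlaps while a player possesses it.
; A timeline adds roll to the blade, then restores the rotation cached on first attack, with a Gate blocking re-swings until it finishes.
; Overlaps with Enemy-tagged BaseEnemy actors roll evasion, then calculate and apply damage, flag the enemy as hit, and send a combat log message for display.
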(event OnComponentBeginOverlap(Blade_Dragon)
  (params (OverlappedComponent :type Primitive%20Component%20Object%20Reference) (OtherActor :type Actor%20Object%20Reference) (OtherComp :type Primitive%20Component%20Object%20Reference) (OtherBodyIndex :type Integer) (bFromSweep :type Boolean) (SweepResult :type Hit%20Result%20Structure%20%28by%20ref%29))
  ;[1 1 1] Blade Collision
  (if (and (Actor|ActorHasTag OtherActor "Enemy") (Utilities|String|Contains (Variables|Default|GetPossessor) "Player"))
    (bind _asbase_enemy (Utilities|Casting|CastToBaseEnemy OtherActor))
    (CallFunction|GetPossessor)
    (Default|CalculateEvasion _asbase_enemy "NewEnumerator1")
    (if (Variables|/Game/Model/EnemyBlueprints/BaseEnemy.BaseEnemy_C|GetEvasionSuccessful _asbase_enemy)
      (CallFunction|CalculateDamage)
      (bind _reduceddamage (Default|ApplyDamage _asbase_enemy (Variables|Default|GetfinalDamageValue) "NewEnumerator1" "0, 0, 0"))
      (Variables|/Game/Model/EnemyBlueprints/BaseEnemy.BaseEnemy_C|SetHitByPlayer _asbase_enemy true)
      (CallFunction|LogDamage (Variables|Default|GetPossessor) (Utilities|GetDisplayName _asbase_enemy) (Utilities|String|EnumtoString (Variables|Default|GetDamageSource)) (Utilities|String|ToString(Float) _reduceddamage) (Utilities|String|EnumtoString (Variables|Default|GetDamageType)))
      (Variables|/Game/Model/EnemyBlueprints/BaseEnemy.BaseEnemy_C|SetDamageSource _asbase_enemy (Utilities|String|EnumtoString (Variables|Default|GetDamageSource))))))

(event Custom|LogDamage
  (params (AttackingUnit :type String) (UnitBeingAttacked :type String) (DamageSource :type String) (AmountOfDamage :type String) (DamageType :type String))
  ;[1 1 1] Log the damage
  (Default|CallDisplayDamage (Utilities|String|Append (Utilities|String|Append (Utilities|String|Append (Utilities|String|Append (Utilities|String|Append (Utilities|String|Append (Utilities|String|Append (Utilities|String|Append (Utilities|String|Append (Utilities|String|Append (Utilities|String|Append AttackingUnit " attacked ") UnitBeingAttacked) "!! 
") "The damage source is ") DamageSource) ". 
") "The amount of damage was ") AmountOfDamage) ". 
") "The damage type was ") DamageType)))

(event Collision|EventActorBeginOverlap
  (params (OtherActor :type Actor%20Object%20Reference)))

(event EventAttack
  (bind _blade_dragon (Variables|Default|GetBlade_Dragon))
  (bind _relativerotation (Variables|/Script/Engine.SceneComponent|GetRelativeRotation _blade_dragon))
  (bind (_roll _pitch _yaw) (Math|Rotator|BreakRotator _relativerotation))
  ;[1 1 1] Swing the sword
  (Utilities|FlowControl|Sequence
    (:then_0
      (Utilities|FlowControl|Gate false :!label _label
        (:Exit
          (Utilities|FlowControl|Sequence
            (:then_0
              (bind _delta (Timeline|Timeline_0 PlayFromStart)
                (:Update
                  (Transformation|SetRelativeRotation (Variables|Default|GetBlade_Dragon) (Math|Rotator|MakeRotator (+ _roll _delta) _pitch _yaw) false false))
                (:Finished
                  (Utilities|FlowControl|Sequence
                    (:then_0
                      (Transformation|SetRelativeRotation (Variables|Default|GetBlade_Dragon) (Variables|Default|GetInitialRotation) false false))
                    (:then_1
                      (goto _label Open))))))
            (:then_1
              (goto _label Toggle))))))
    (:then_1
      (Utilities|FlowControl|DoOnce false
        (:Completed
          (Variables|Default|SetInitialRotation (Variables|/Script/Engine.SceneComponent|GetRelativeRotation (Variables|Default|GetBlade_Dragon))))))))

(fn ConstructionScript)